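; Gianni is a player-controlled pawn Blueprint that handles basic movement and look input.
; Avanti_indetro and destra_sinistra axes add movement along the control rotation's forward and right vectors, with pitch left in.
; The rotation axis names are crossed relative to their effect: rotazione_su_giu (up/down) drives yaw and rotazione_dx_sx (right/left) drives pitch.
; BeginPlay, overlap, Tick and the construction script are empty.
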(event EventBeginPlay)

(event Collision|EventActorBeginOverlap
  (params (OtherActor :type Actor%20Object%20Reference)))

(event EventTick
  (params (DeltaSeconds :type Float%20%28single-precision%29)))

(event Input|AxisEvents|InputAxisdestra_sinistra
  (params (AxisValue :type Float%20%28single-precision%29))
  ;[1 1 1] WASD
  (Pawn|Input|AddMovementInput (Math|Vector|GetRightVector (Pawn|GetControlRotation :!class /Script/Engine.Pawn)) AxisValue false))

(event Input|AxisEvents|InputAxisAvanti_indietro
  (params (AxisValue :type Float%20%28single-precision%29))
  ;[1 1 1] WASD
  (Pawn|Input|AddMovementInput (Math|Vector|GetForwardVector (Pawn|GetControlRotation :!class /Script/Engine.Pawn)) AxisValue false))

(event Input|AxisEvents|InputAxisrotazione_su_giu
  (params (AxisValue :type Float%20%28single-precision%29))
  (Pawn|Input|AddControllerYawInput AxisValue))

(event Input|AxisEvents|InputAxisrotazione_dx_sx
  (params (AxisValue :type Float%20%28single-precision%29))
  (Pawn|Input|AddControllerPitchInput AxisValue))

(fn ConstructionScript)